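; Player controller that drives BP_Character from Enhanced Input.
; BeginPlay caches player 0's pawn as MainCharacter and adds IMC_MappingContext to the input subsystem.
; IA_Move feeds StartMoving, which adds movement input along a right vector built only from control rotation roll, scaled by the axis value, with identical logic in both sign branches.
; IA_Jump is bound but empty.
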(event `self.ReceiveBeginPlay`
  (bind _returnvalue (pcsubsystem `EnhancedInputLocalPlayerSubsystem` self))
  (`|ExecutionSequence`
    (:`then_0`
      (bind _asbp_character (cast `/Game/Blueprints/BP_Character` (`GameplayStatics.GetPlayerPawn` 0)))
      (set `self.Main Character` _asbp_character))
    (:`then_1`
      (`/Engine/EditorBlueprintResources/StandardMacros.IsValid` _returnvalue
        (:`Is Valid`
          (`EnhancedInputSubsystemInterface.AddMappingContext` _returnvalue "/Game/Inputs/IMC_MappingContext.IMC_MappingContext" 0 (struct)) ; If valide, this controller will use this mapping context
        )))))

(event `EnhancedInput|/Game/Inputs/IA_Move`
  (params (ActionValue :type "Float (double-precision)") (ElapsedSeconds :type "Float (double-precision)") (TriggeredSeconds :type "Float (double-precision)") (InputAction :type "InputAction Object Reference" :default "/Game/Inputs/IA_Move.IA_Move"))
  (:`Triggered`
    (`self.StartMoving` ActionValue)))

(event `EnhancedInput|/Game/Inputs/IA_Jump`
  (params (ActionValue :type Boolean) (ElapsedSeconds :type "Float (double-precision)") (TriggeredSeconds :type "Float (double-precision)") (InputAction :type "InputAction Object Reference" :default "/Game/Inputs/IA_Jump.IA_Jump")))

(fn `StartMoving`
  (params (`Axis Value` :type "Float (double-precision)"))
  (bind _main_character (`self.Main Character`))
  (bind _returnvalue_roll (`KismetMathLibrary.BreakRotator` (`Pawn.GetControlRotation` _main_character)))
  (bind _returnvalue (`KismetMathLibrary.GetRightVector` (`KismetMathLibrary.MakeRotator` _returnvalue_roll)))
  (if (> `Axis Value` 0.0)
    (`Pawn.AddMovementInput` _main_character _returnvalue `Axis Value` false)
    (else
      (`Pawn.AddMovementInput` _main_character _returnvalue `Axis Value` false))))

(fn `UserConstructionScript`)